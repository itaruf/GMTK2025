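; Calendar prop that keeps its displayed day in step with the game's loop progress.
; On BeginPlay it subscribes to the loop subsystem's end and continue events, then calls AdvanceDay at iteration zero.
; Continuing a loop advances to the reported iteration, while a failed loop end resets to zero and a successful one changes nothing.
; AdvanceDay receives the subsystem's total iteration count each time and is defined outside these graphs.
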(event `self.ReceiveBeginPlay`
  (add `LoopSubsystem.OnLoopEnd` (subsystem `LoopSubsystem`) (`|CreateDelegate` :!event `Event Loop End`))
  (add `LoopSubsystem.OnLoopContinue` (subsystem `LoopSubsystem`) (`|CreateDelegate` :!event `Event Loop Continue`))
  (`self.AdvanceDay` 0 (`LoopSubsystem.GetTotalIterations` (subsystem `LoopSubsystem`))))

(event `Event Loop End`
  (params (bSuccess :type Boolean))
  (if (not bSuccess)
    (`self.AdvanceDay` 0 (`LoopSubsystem.GetTotalIterations` (subsystem `LoopSubsystem`)))))

(event `Event Loop Continue`
  (params (Iteration :type Integer))
  (`self.AdvanceDay` Iteration (`LoopSubsystem.GetTotalIterations` (subsystem `LoopSubsystem`))))

(fn `UserConstructionScript`)
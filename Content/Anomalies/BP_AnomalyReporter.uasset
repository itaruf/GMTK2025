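; BP_AnomalyReporter is the in-world Yes/No choice point where the player reports an anomaly in the loop.
; Overlapping Yes reports to the loop subsystem, except on iteration zero, where it continues the loop like No.
; Either choice sets the controller's Transitioning flag to block repeat triggers.
; A widget component shows the prompt, registered with the player HUD and switched between initial and anomaly text by loop events.
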(event `self.ReceiveBeginPlay`
  (bind _returnvalue (subsystem `LoopSubsystem`))
  (bind _asbp_third_person_player_controller (cast `/Game/ThirdPerson/Blueprints/BP_ThirdPersonPlayerController` (`GameplayStatics.GetPlayerController` 0)))
  (bind _output_get (set `self.PlayerController` _asbp_third_person_player_controller))
  (add `/Game/ThirdPerson/Blueprints/BP_ThirdPersonPlayerController.OnInitEnded` _output_get (`|CreateDelegate` :!event `Init`))
  (add `LoopSubsystem.OnLoopContinue` _returnvalue (`|CreateDelegate` :!event `Event Loop Continue`))
  (add `LoopSubsystem.OnLoopEnd` _returnvalue (`|CreateDelegate` :!event `Event Loop End`)))

(event `Init`
  (bind _asw_anomaly_confirmation (cast `/Game/UI/W_AnomalyConfirmation` (`WidgetComponent.GetUserWidgetObject` (`self.AnomalyConfirmationWidgetComp`))))
  (bind _output_get (set `/Game/UI/HUD_Player.AnomalyConfirmationWidget` _asw_anomaly_confirmation (`/Game/ThirdPerson/Blueprints/BP_ThirdPersonPlayerController.HUD Player` (`self.PlayerController`))))
  (`TextBlock.SetText` (`/Game/UI/W_AnomalyConfirmation.AnomalyPromptText` (`/Game/UI/HUD_Player.AnomalyConfirmationWidget` (`/Game/ThirdPerson/Blueprints/BP_ThirdPersonPlayerController.HUD Player` (`self.PlayerController`)))) (`self.AnomalyInitialText`))
  (`Widget.SetVisibility` _output_get "Visible"))

(event `Event Anomaly Confirmation`
  (params (bConfirmed :type Boolean)))

(event `self.AmalaBoxCollision.OnComponentBeginOverlap`
  (params (OverlappedComponent :type "PrimitiveComponent Object Reference") (OtherActor :type "Actor Object Reference") (OtherComp :type "PrimitiveComponent Object Reference") (OtherBodyIndex :type Integer) (bFromSweep :type Boolean) (SweepResult :type "HitResult Structure (by ref)"))
  (if (== OtherActor (`GameplayStatics.GetPlayerPawn` 0))
    _))

(event `self.AmalaBoxCollision.OnComponentEndOverlap`
  (params (OverlappedComponent :type "PrimitiveComponent Object Reference") (OtherActor :type "Actor Object Reference") (OtherComp :type "PrimitiveComponent Object Reference") (OtherBodyIndex :type Integer))
  (if (== OtherActor (`GameplayStatics.GetPlayerPawn` 0))
    _))

(event `self.YesBoxCollision.OnComponentBeginOverlap`
  (params (OverlappedComponent :type "PrimitiveComponent Object Reference") (OtherActor :type "Actor Object Reference") (OtherComp :type "PrimitiveComponent Object Reference") (OtherBodyIndex :type Integer) (bFromSweep :type Boolean) (SweepResult :type "HitResult Structure (by ref)"))
  (if (and (== OtherActor (`GameplayStatics.GetPlayerPawn` 0)) (not (`/Game/ThirdPerson/Blueprints/BP_ThirdPersonPlayerController.Transitioning` (`self.PlayerController`))))
    (`KismetSystemLibrary.PrintString` "YES")
    (if (== (`LoopSubsystem.GetCurrentIteration` (subsystem `LoopSubsystem`)) 0)
      (`LoopSubsystem.ContinueLoop` (subsystem `LoopSubsystem`))
      (else
        (`LoopSubsystem.ReportAnomaly` (subsystem `LoopSubsystem`))))
    (set `/Game/ThirdPerson/Blueprints/BP_ThirdPersonPlayerController.Transitioning` true (`self.PlayerController`) :!label _label)))

(event `self.NoBoxCollision.OnComponentBeginOverlap`
  (params (OverlappedComponent :type "PrimitiveComponent Object Reference") (OtherActor :type "Actor Object Reference") (OtherComp :type "PrimitiveComponent Object Reference") (OtherBodyIndex :type Integer) (bFromSweep :type Boolean) (SweepResult :type "HitResult Structure (by ref)"))
  (if (and (not (`/Game/ThirdPerson/Blueprints/BP_ThirdPersonPlayerController.Transitioning` (`self.PlayerController`))) (== OtherActor (`GameplayStatics.GetPlayerPawn` 0)))
    (`KismetSystemLibrary.PrintString` "NO")
    (`LoopSubsystem.ContinueLoop` (subsystem `LoopSubsystem`))
    (goto _label)))

(event `Event Loop Continue`
  (params (Iteration :type Integer))
  (`TextBlock.SetText` (`/Game/UI/W_AnomalyConfirmation.AnomalyPromptText` (`/Game/UI/HUD_Player.AnomalyConfirmationWidget` (`/Game/ThirdPerson/Blueprints/BP_ThirdPersonPlayerController.HUD Player` (`self.PlayerController`)))) (`self.AnomalyPromptText`)))

(event `Event Loop End`
  (params (bSuccess :type Boolean))
  (if (not bSuccess)
    (`TextBlock.SetText` (`/Game/UI/W_AnomalyConfirmation.AnomalyPromptText` (`/Game/UI/HUD_Player.AnomalyConfirmationWidget` (`/Game/ThirdPerson/Blueprints/BP_ThirdPersonPlayerController.HUD Player` (`self.PlayerController`)))) (`self.AnomalyInitialText`))))

(fn `UserConstructionScript`)